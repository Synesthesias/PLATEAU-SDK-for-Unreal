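; Blueprint function library for PLATEAU city models, providing a line trace that finds the city object between a start and end point.
; It runs a complex multi line trace on the Visibility channel with timed debug drawing, then skips hidden components.
; The first visible PLATEAU city object group hit resolves its primary city object from the hit, returned with a success flag.
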(fn LineTraceCityObject
  (params (Start :type Vector) (End :type Vector))
  (bind _outhits (Collision|MultiLineTraceByChannel 0 Start End "TraceTypeQuery1" true 0 "ForDuration"))
  (bind _array_element (Utilities|Array|ForEachLoopwithBreak _outhits :!label _label)
    (:LoopBody
      (if (and (Rendering|IsVisible (.HitComponent (Collision|BreakHitResult _array_element))) (!= true false))
        (bind _asplateaucity_object_group (Utilities|Casting|CastToPLATEAUCityObjectGroup (.HitComponent (Collision|BreakHitResult _array_element)))
          (:then
            (bind _returnvalue (Class|PLATEAUCityObjectGroup|GetPrimaryCityObjectbyRaycast _asplateaucity_object_group _array_element))
            (LocalVariables|SetCityObj _returnvalue)
            (LocalVariables|SetHitResult true)
            (goto _label Break))
          (:CastFailed
            (LocalVariables|SetHitResult false)))
        (else
          (LocalVariables|SetHitResult false))))
    (:Completed
      (return (LocalVariables|GetHitResult) (LocalVariables|GetCityObj)))))